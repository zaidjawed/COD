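; Base weapon Blueprint handling hitscan firing, ammo, reloading and weapon data getters.
; FireWeapon spends a bullet, plays montage and sound, then line-traces from the passed camera, spawning impact effects and damaging only Enemy-surface hits.
; ReloadWeapon refills ammo from WeaponStats on a montage notify.
; Both push ammo counts to WBP_WeaponStats, found via a widget class search, and the trace leaves debug drawing enabled.
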(event EventBeginPlay)

(event Collision|EventActorBeginOverlap
  (params (OtherActor :type Actor%20Object%20Reference)))

(event EventTick
  (params (DeltaSeconds :type Float%20%28single-precision%29)))

(event EventReloadWeapon
  ;[1 1 1] Reload
  (Animation|Montage|PlayMontage (Variables|Default|GetMesh%20Weapon) (Variables|Montage|GetWeaponReloadMontage)
    (:OnNotifyBegin
      (Variables|Stats|SetCurrentBullet (.MaxBullet (Utilities|Struct|BreakS_WeaponStats (Variables|Stats|GetWeaponStats))))
      (CallFunction|UpdateWeaponAmmoWidget))))

(event EventFireWeapon
  (params (Camera :type Camera%20Component%20Object%20Reference))
  (bind _returnvalue (Transformation|GetWorldLocation Camera))
  ;[1 1 1] Fire Event
  (if (> (Variables|Stats|GetCurrentBullet) 0)
    (Variables|Stats|SetCurrentBullet (- (Variables|Stats|GetCurrentBullet) 1))
    (Animation|Montage|PlayMontage (Variables|Default|GetMesh%20Weapon) (Variables|Montage|GetWeaponFireMontage)
      (:then
        (Audio|SpawnSoundatLocation (Variables|Sound|GetFireSoundCue) (Transformation|GetSocketLocation (Variables|Default|GetMesh%20Weapon) "SOCKET_Muzzle") "0, 0, 0" 1.0 (Class|GameplayStatics|GetGlobalTimeDilation) 0.0 0 0)
        (CallFunction|UpdateWeaponAmmoWidget)
        (bind (_outhit _returnvalue_2) (Collision|LineTraceByChannel _returnvalue (+ _returnvalue (* (Math|Vector|GetForwardVector (Transformation|GetWorldRotation Camera)) 99999.0)) "TraceTypeQuery1" false 0 "ForDuration" true "(R=1.000000,G=0.000000,B=0.000000,A=1.000000)" "(R=0.000000,G=1.000000,B=0.000000,A=1.000000)" 3.0))
        (if _returnvalue_2
          (Rendering|Decal|SpawnDecalatLocation "/Game/Effects/MI_Decal_Bullet_Concrete.MI_Decal_Bullet_Concrete" "5.000000,5.000000,5.000000" (.ImpactPoint (Collision|BreakHitResult _outhit)) (Math|Conversions|RotationFromXVector (.ImpactNormal (Collision|BreakHitResult _outhit))) 0.0)
          (Effects|SpawnEmitteratLocation "/Game/Effects/PS_Impact.PS_Impact" (.ImpactPoint (Collision|BreakHitResult _outhit)) (Math|Conversions|RotationFromXVector (.ImpactNormal (Collision|BreakHitResult _outhit))) "0.800000,0.800000,0.800000")
          (Audio|SpawnSoundatLocation "/Game/MetaSound/MSP_BulletImpact.MSP_BulletImpact" (.ImpactPoint (Collision|BreakHitResult _outhit)) "0, 0, 0" 1.0 1.0 0.0 0 0)
          (switch Utilities|FlowControl|Switch|SwitchonEPhysicalSurface (Variables|/Script/PhysicsCore.PhysicalMaterial|GetSurfaceType (.PhysMat (Collision|BreakHitResult _outhit)))
            (:SurfaceType1
              (Game|Damage|ApplyDamage (.HitActor (Collision|BreakHitResult _outhit)) (.Damage (Utilities|Struct|BreakS_WeaponStats (Variables|Stats|GetWeaponStats))) 0 0))))))))

(event EventStopAnimMontage
  ;[1 1 1] Stop montage
  (Animation|Montage|MontageStop (Components|SkeletalMesh|GetAnimInstance (Variables|Default|GetMesh%20Weapon)) 0.0 0))

(fn ConstructionScript)

(fn UpdateWeaponAmmoWidget
  (bind _foundwidgets (Widget|GetAllWidgetsOfClass "/Game/Widget/WBP_WeaponStats.WBP_WeaponStats_C" true))
  (LocalVariables|SetStatsWidgetRef (Utilities|Array|Get(acopy) _foundwidgets))
  (Class|BPIWidgetWeaponStats|ReceiveCurrentBullets(Message) (LocalVariables|GetStatsWidgetRef) (Utilities|Text|ToText(Integer) (Variables|Stats|GetCurrentBullet)))
  (Class|BPIWidgetWeaponStats|ReceiveMaxBullets(Message) (LocalVariables|GetStatsWidgetRef) (Utilities|Text|ToText(Integer) (.MaxBullet (Utilities|Struct|BreakS_WeaponStats (Variables|Stats|GetWeaponStats))))))

(fn GetCurrentBullet
  (return (Variables|Stats|GetCurrentBullet)))

(fn GetFireMontage
  (return (Variables|Montage|GetFireMontage)))

(fn GetInspectMontage
  (return (Variables|Montage|GetInspectMontage)))

(fn GetIsWeaponEmpty
  (return (== (Variables|Stats|GetCurrentBullet) 0)))

(fn GetIsWeaponFull
  (return (== (Variables|Stats|GetCurrentBullet) (.MaxBullet (Utilities|Struct|BreakS_WeaponStats (Variables|Stats|GetWeaponStats))))))

(fn GetReloadMontage
  (return (Variables|Montage|GetReloadMontage)))

(fn GetWeaponIcon
  (bind _weaponsize (Variables|Widget|GetWeaponSize))
  (bind (_x _y) (Math|Vector2D|BreakVector2D _weaponsize))
  (return (Variables|Widget|GetWeaponIcon) (Math|Float|Truncate _x) (Math|Float|Truncate _y)))

(fn GetWeaponStats
  (return (Variables|Stats|GetWeaponStats)))