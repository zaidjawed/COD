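; Base weapon Blueprint handling firing, reloading, ammo tracking and getters for montages, icon and stats.
; Firing spends a bullet, plays the weapon montage and sound, then line traces from the muzzle socket toward a distant camera-forward point, spawning impact decal, particles and sound without applying damage.
; Reload refills ammo on the montage's notify.
; Both push counts to the W_WeaponStats widget, found by class search.
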(event EventBeginPlay)

(event Collision|EventActorBeginOverlap
  (params (OtherActor :type Actor%20Object%20Reference)))

(event EventTick
  (params (DeltaSeconds :type Float%20%28single-precision%29)))

(event EventReloadWeapon
  (Animation|Montage|PlayMontage (Variables|Default|GetMesh%20Weapon) (Variables|Montage|GetWeaponReloadMontage)
    (:OnNotifyBegin
      (Variables|Stats|SetCurrentBullet (.MaxBullet (Utilities|Struct|BreakS_WeaponStats (Variables|Stats|GetWeaponStats))))
      (CallFunction|UpdateWeaponAmmoWidget))))

(event EventFireWeapon
  (bind _returnvalue (Game|GetPlayerCameraManager 0))
  (if (> (Variables|Stats|GetCurrentBullet) 0)
    (Variables|Stats|SetCurrentBullet (- (Variables|Stats|GetCurrentBullet) 1))
    (Animation|Montage|PlayMontage (Variables|Default|GetMesh%20Weapon) (Variables|Montage|GetWeaponFireMontage)
      (:then
        (Audio|SpawnSoundatLocation "/Game/MetaSound/MSP_RifleFire.MSP_RifleFire" (Transformation|GetSocketLocation (Variables|Default|GetMesh%20Weapon) "SOCKET_Muzzle") "0, 0, 0" 1.0 1.0 0.0 0 0)
        (CallFunction|UpdateWeaponAmmoWidget)
        (bind (_outhit _returnvalue_2) (Collision|LineTraceByChannel (.Location (Math|Transform|BreakTransform (Transformation|GetSocketTransform (Variables|Default|GetMesh%20Weapon) "SOCKET_Muzzle" "RTS_World"))) (+ (Camera|GetCameraLocation _returnvalue) (* (Math|Vector|GetForwardVector (Camera|GetCameraRotation _returnvalue)) 99999.0)) "TraceTypeQuery1" false 0 "None" true "(R=1.000000,G=0.000000,B=0.000000,A=1.000000)" "(R=0.000000,G=1.000000,B=0.000000,A=1.000000)" 2.0))
        (if _returnvalue_2
          (Rendering|Decal|SpawnDecalatLocation "/Game/Art/Effects/MI_Decal_Bullet_Concrete.MI_Decal_Bullet_Concrete" "5.000000,5.000000,5.000000" (.ImpactPoint (Collision|BreakHitResult _outhit)) (Math|Conversions|RotationFromXVector (.ImpactNormal (Collision|BreakHitResult _outhit))) 0.0)
          (Effects|SpawnEmitteratLocation "/Game/Art/Effects/PS_Impact.PS_Impact" (.ImpactPoint (Collision|BreakHitResult _outhit)) (Math|Conversions|RotationFromXVector (.ImpactNormal (Collision|BreakHitResult _outhit))) "0.800000,0.800000,0.800000")
          (Audio|SpawnSoundatLocation "/Game/MetaSound/MSP_BulletImpact.MSP_BulletImpact" (.ImpactPoint (Collision|BreakHitResult _outhit)) "0, 0, 0" 1.0 1.0 0.0 0 0))))))

(event EventStopAnimMontage
  (Animation|Montage|MontageStop (Components|SkeletalMesh|GetAnimInstance (Variables|Default|GetMesh%20Weapon)) 0.0 0))

(fn ConstructionScript)

(fn UpdateWeaponAmmoWidget
  (bind _foundwidgets (Widget|GetAllWidgetsOfClass "/Game/Widget/W_WeaponStats.W_WeaponStats_C" true))
  (LocalVariables|SetStatsWidgetRef (Utilities|Array|Get(acopy) _foundwidgets))
  (Class|ABPWidget|ReceiveCurrentBullets(Message) (LocalVariables|GetStatsWidgetRef) (Utilities|Text|ToText(Integer) (Variables|Stats|GetCurrentBullet)))
  (Class|ABPWidget|ReceiveMaxBullets(Message) (LocalVariables|GetStatsWidgetRef) (Utilities|Text|ToText(Integer) (.MaxBullet (Utilities|Struct|BreakS_WeaponStats (Variables|Stats|GetWeaponStats))))))

(fn GetCurrentBullet
  (return (Variables|Stats|GetCurrentBullet)))

(fn GetFireMontage
  (return (Variables|Montage|GetFireMontage)))

(fn GetInspectMontage
  (return (Variables|Montage|GetInspectMontage)))

(fn GetIsWeaponEmpty
  (return (== (Variables|Stats|GetCurrentBullet) 0)))

(fn GetIsWeaponFull
  (return (== (Variables|Stats|GetCurrentBullet) (.MaxBullet (Utilities|Struct|BreakS_WeaponStats (Variables|Stats|GetWeaponStats))))))

(fn GetReloadMontage
  (return (Variables|Montage|GetReloadMontage)))

(fn GetWeaponIcon
  (bind _weaponsize (Variables|Widget|GetWeaponSize))
  (bind (_x _y) (Math|Vector2D|BreakVector2D _weaponsize))
  (return (Variables|Widget|GetWeaponIcon) (Math|Float|Truncate _x) (Math|Float|Truncate _y)))

(fn GetWeaponStats
  (return (Variables|Stats|GetWeaponStats)))