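; BP_EnemyBase is a base enemy that periodically shoots at the player and is destroyed when damage depletes its health.
; A looping timer set on BeginPlay fires Attack, which snaps the actor's rotation toward the player, then spawns a BP_Projectile at the rifle's muzzle socket.
; Projectile rotation is computed from the actor's location to the player's rather than from the muzzle.
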(event Custom|Attack
  ;[1 1 1] Attack
  (CallFunction|LookatPlayer)
  (Game|SpawnActorfromClass "/Game/Enemy/BP_Projectile.BP_Projectile_C" (Math|Transform|MakeTransform (.location (Transformation|GetSocketTransform (Variables|Default|GetRifle) "SOCKET_Muzzle" "RTS_World")) (Math|Rotator|FindLookatRotation (Transformation|GetActorLocation) (Transformation|GetActorLocation (Game|GetPlayerCharacter 0))) "1.000000,1.000000,1.000000") "AlwaysSpawn" "MultiplyWithRoot" 0 0))

(event Custom|LookAtPlayer
  ;[1 1 1] Look at player
  (Transformation|SetActorRotation (Math|Rotator|FindLookatRotation (Transformation|GetActorLocation) (Transformation|GetActorLocation (Game|GetPlayerCharacter 0)))))

(event EventBeginPlay
  ;[0 1 0.2822] Begin play
  (Utilities|Time|SetTimerbyEvent (delegate Custom|Attack) (Variables|Default|GetAttackDelay) true))

(event Game|Damage|EventAnyDamage
  (params (Damage :type Float%20%28single-precision%29) (DamageType :type Damage%20Type%20Object%20Reference) (InstigatedBy :type Controller%20Object%20Reference) (DamageCauser :type Actor%20Object%20Reference))
  ;[1 1 1] Any damage
  (if (<= (- (Variables|Default|GetHealth) Damage) 0.0)
    (Actor|DestroyActor)
    (else
      (Variables|Default|SetHealth (- (Variables|Default|GetHealth) Damage)))))

(fn ConstructionScript)