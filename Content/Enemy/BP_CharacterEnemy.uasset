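; Enemy character Blueprint that arms itself and can fire at the player.
; BeginPlay calls SetupWeapon and the Attack event calls Fire, with neither function's logic defined in this graph.
; LookatPlayer snaps the actor's full rotation toward player character 0 via FindLookAtRotation and prints the player's location for debugging.
; Tick is empty, so nothing here triggers aiming or attacking, and construction only runs the parent script.
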(event EventBeginPlay
  (CallFunction|SetupWeapon))

(event EventAttack
  (CallFunction|Fire))

(event EventLookatPlayer
  (bind _returnvalue (Game|GetPlayerCharacter 0))
  (bind _returnvalue_2 (Transformation|GetActorLocation _returnvalue))
  (Development|PrintString "Player Location" true true "(R=0.000000,G=0.660000,B=1.000000,A=1.000000)" 2.0 "x")
  (Development|PrintString (Utilities|String|ToString(Vector) _returnvalue_2) true true "(R=0.000000,G=0.660000,B=1.000000,A=1.000000)" 2.0 "Player Location")
  (Transformation|SetActorRotation (Math|Rotator|FindLookatRotation (Transformation|GetActorLocation) _returnvalue_2)))

(event EventTick
  (params (DeltaSeconds :type Float%20%28single-precision%29)))

(fn ConstructionScript
  (|CallParentFunction))